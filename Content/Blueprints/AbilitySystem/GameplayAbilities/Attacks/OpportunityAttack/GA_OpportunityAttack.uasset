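; Gameplay ability for an opportunity attack, which damages the avatar character's current CombatTarget when activated.
; It builds a spec from the damage effect class and applies it from the source's ability system component to the target's, unless the target has the ImmuneToOpportunityAction tag.
; The ability ends itself only in the immune case, and a debug sphere is drawn at the target in both cases.
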(event `self.K2_ActivateAbility`
  (bind _ashexplore_character_base (cast `HexploreCharacterBase` (`self.GetAvatarActorFromActorInfo`)))
  (set `self.Source` _ashexplore_character_base)
  (set `self.Target` (`HexploreCharacterBase.CombatTarget` (`self.Source`)))
  (`self.MakeSpecAndApplyToTarget`)
  (`KismetSystemLibrary.DrawDebugSphere` (`Actor.K2_GetActorLocation` (`self.Target`)) 50.0 12 (struct :`R` 0.546875 :`B` 0.081917 :`A` 1.0) 1.0))

(fn `MakeSpecAndApplyToTarget`
  (bind _returnvalue (`AbilitySystemBlueprintLibrary.GetAbilitySystemComponent` (`self.Source`)))
  (bind _returnvalue_2 (`AbilitySystemBlueprintLibrary.GetAbilitySystemComponent` (`self.Target`)))
  (if (`GameplayTagAssetInterface.HasMatchingGameplayTag` _returnvalue_2 (struct :`TagName` "Status.General.ImmuneToOpportunityAction"))
    (`self.K2_EndAbility`)
    (else
      (`AbilitySystemComponent.BP_ApplyGameplayEffectSpecToTarget` _returnvalue (`AbilitySystemComponent.MakeOutgoingSpec` :`self` _returnvalue :`GameplayEffectClass` (`self.DamageEffectClass`)) _returnvalue_2))))