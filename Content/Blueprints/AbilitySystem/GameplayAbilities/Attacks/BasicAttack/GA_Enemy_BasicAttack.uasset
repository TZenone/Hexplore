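; Gameplay ability for an enemy's basic attack against the avatar character's CombatTarget.
; On activation it checks that the target is within AbilityRange, then commits the stamina cost and applies DamageEffectClass to the target's ability system immediately.
; EndAbility is called only when the range or cost check fails, not after a successful hit.
; Attack montage and gameplay-event wait nodes are unconnected, with enemy animation left as a TODO.
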(event `self.K2_ActivateAbility`
  (bind _ashexplore_character_base (cast `HexploreCharacterBase` (`self.GetAvatarActorFromActorInfo`)))
  (set `self.Source` _ashexplore_character_base)
  (set `self.Target` (`HexploreCharacterBase.CombatTarget` (`self.Source`)))
  ;[0.2993 1 0.1719] Check range
  (bind _returnvalue (`self.IsTargetInRange` (`self.AbilityRange`) (`self.Source`) (`self.Target`)))
  (if _returnvalue
    ;[0.2993 1 0.1719] Check Stamina
    (bind _returnvalue_2 (`self.K2_CommitAbilityCost` false))
    (if _returnvalue_2
      (`self.MakeSpecAndApplyToTarget`)
      (else
        (`self.K2_EndAbility`)))
    (else
      (`self.K2_EndAbility`))))

(fn `IsTargetInRange`
  (params (AbilityRange :type "Float (single-precision)") (Character :type "Actor Object Reference") (Target :type "Actor Object Reference"))
  (returns (ReturnValue :type Boolean))
  (return (<= (`Actor.GetDistanceTo` Target Character) AbilityRange)))

(fn `MakeSpecAndApplyToTarget`
  (bind _returnvalue (`AbilitySystemBlueprintLibrary.GetAbilitySystemComponent` (`self.Source`)))
  (`AbilitySystemComponent.BP_ApplyGameplayEffectSpecToTarget` _returnvalue (`AbilitySystemComponent.MakeOutgoingSpec` :`self` _returnvalue :`GameplayEffectClass` (`self.DamageEffectClass`)) (`AbilitySystemBlueprintLibrary.GetAbilitySystemComponent` (`self.Target`))))