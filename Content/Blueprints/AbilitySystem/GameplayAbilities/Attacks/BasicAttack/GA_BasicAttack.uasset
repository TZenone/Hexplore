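; Basic attack gameplay ability that strikes the Hexplore character's current combat target.
; On activation it checks range (drawing a debug sphere) and commits the ability cost, ending if either fails.
; It then plays the attack montage and waits for the auto-attack gameplay event to apply the damage effect spec to the target.
; The successful attack path never calls EndAbility.
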(event `self.K2_ActivateAbility`
  (bind _asbp_hexplore_character (cast `/Game/Blueprints/Character/Hexplore/BP_HexploreCharacter` (`self.GetAvatarActorFromActorInfo`)))
  (set `self.Source` _asbp_hexplore_character)
  (set `self.Target` (`HexploreCharacterBase.CombatTarget` (`self.Source`)))
  ;[0.2993 1 0.1719] Check range
  (bind _returnvalue (`self.IsTargetInRange` (`self.AbilityRange`) (`self.Source`) (`self.Target`)))
  (if _returnvalue
    ;[0.2993 1 0.1719] Check Stamina
    (bind _returnvalue_2 (`self.K2_CommitAbilityCost` false))
    (if _returnvalue_2
      (`AbilityTask_PlayMontageAndWait.CreatePlayMontageAndWaitProxy` "None" "/Game/Assets/Character/Animations/Attacks/OneHanded/AM_Attack.AM_Attack"
        (:`then`
          (`AbilityTask_WaitGameplayEvent.WaitGameplayEvent` (struct :`TagName` "Event.Montage.AutoAttack") null true
            (:`EventReceived`
              (`self.MakeSpecAndApplyToTarget`)))))
      (else
        (`self.K2_EndAbility`)))
    (else
      (`self.K2_EndAbility`))))

(fn `IsTargetInRange`
  (params (AbilityRange :type "Float (single-precision)") (Character :type "Actor Object Reference") (Target :type "Actor Object Reference"))
  (returns (ReturnValue :type Boolean))
  (bind _returnvalue_location (`KismetMathLibrary.BreakTransform` (`Actor.GetTransform` Character)))
  (`KismetSystemLibrary.DrawDebugSphere` _returnvalue_location AbilityRange 12 (struct :`R` 1.0 :`G` 0.374892 :`B` 0.443317 :`A` 1.0) 1.0)
  (return (<= (`Actor.GetDistanceTo` Target Character) AbilityRange)))

(fn `MakeSpecAndApplyToTarget`
  (bind _returnvalue (`AbilitySystemBlueprintLibrary.GetAbilitySystemComponent` (`self.Source`)))
  (`AbilitySystemComponent.BP_ApplyGameplayEffectSpecToTarget` _returnvalue (`AbilitySystemComponent.MakeOutgoingSpec` :`self` _returnvalue :`GameplayEffectClass` (`self.DamageEffectClass`)) (`AbilitySystemBlueprintLibrary.GetAbilitySystemComponent` (`self.Target`))))