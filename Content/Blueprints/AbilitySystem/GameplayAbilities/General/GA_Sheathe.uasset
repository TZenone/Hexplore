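; Gameplay ability that toggles the avatar character's weapon between sheathed and drawn, using one-handed-and-shield montages.
; Branches on the current sheathed state to play the matching montage and wait for its gameplay event tag.
; That event flips the sheathed state and ends the ability.
; Montage completion or interruption also leads into the event wait rather than ending the ability.
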(event `self.K2_ActivateAbility`
  (bind _ashexplore_character_base (cast `HexploreCharacterBase` (`self.GetAvatarActorFromActorInfo`)))
  (bind _output_get (set `self.OwningBaseCharacter` _ashexplore_character_base))
  (if (`HexploreCharacterBase.bWeaponIsSheathed` _output_get)
    (`AbilityTask_PlayMontageAndWait.CreatePlayMontageAndWaitProxy` "None" "/Game/Assets/Animations/AM_Unsheathe_1HShield.AM_Unsheathe_1HShield"
      (:`then`
        _)
      (:`OnCompleted`
        _)
      (:`OnInterrupted`
        _))
    (`AbilityTask_WaitGameplayEvent.WaitGameplayEvent` (struct :`TagName` "Event.Montage.Unsheathe") null
      (:`EventReceived`
        (`HexploreCharacterBase.SetWeaponSheathed` (`self.OwningBaseCharacter`) false)
        (`self.K2_EndAbility`)))
    (else
      (`AbilityTask_PlayMontageAndWait.CreatePlayMontageAndWaitProxy` "None" "/Game/Assets/Animations/AM_Sheathe_1HShield.AM_Sheathe_1HShield"
        (:`then`
          _)
        (:`OnCompleted`
          _)
        (:`OnInterrupted`
          _))
      (`AbilityTask_WaitGameplayEvent.WaitGameplayEvent` (struct :`TagName` "Event.Montage.Sheathe") null
        (:`EventReceived`
          (`HexploreCharacterBase.SetWeaponSheathed` (`self.OwningBaseCharacter`) true)
          (`self.K2_EndAbility`))))))